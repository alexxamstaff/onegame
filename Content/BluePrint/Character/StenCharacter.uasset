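; Sten is a 2D flipbook enemy character with randomized starting health, skin and walk speed that hurts the Kenny player on contact.
; It wanders to random points along the X axis and moves to Kenny's location when pawn sensing spots him.
; Capsule overlap starts a looping timer that applies damage every second until overlap ends.
; Health regenerates on Tick, and lethal damage destroys the actor.
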(event `self.ReceiveBeginPlay`
  ;[1 1 1] HealtSystem
  (set `self.CurrentHealth` (`KismetMathLibrary.RandomFloatInRange` 20.0 (`self.MaxHealth`)))
  ;[1 1 1] WalkToPlayer
  (`self.StenWalk`)
  ;[1 1 1] SetSkin
  (`PaperFlipbookComponent.SetFlipbook` (`self.Sprite`) (`KismetArrayLibrary.Array_Get` (`self.SpriteArray`) (`KismetMathLibrary.RandomIntegerInRange` 0 2)))
  ;[1 1 1] SpeedWalk
  (set `CharacterMovementComponent.MaxWalkSpeed` (`KismetMathLibrary.RandomFloatInRange` 20.0 500.0) (`self.CharacterMovement`)))

(event `self.ReceiveTick`
  (params (DeltaSeconds :type "Float (single-precision)"))
  ;[1 1 1] HealtSystem
  (`self.ChangeHealth`))

(event `self.PawnSensing.OnSeePawn`
  (params (Pawn :type "Pawn Object Reference"))
  ;[1 1 1] WalkToPlayer
  (bind _askenny_character (cast `/Game/BluePrint/Character/KennyCharacter` Pawn))
  (`|AIMoveTo` self (`self.K2_GetActorLocation` _askenny_character) null 5.0
    (:`OnSuccess`
      _)
    (:`OnFail`
      _))
  (`self.StenWalk`))

(event `self.ReceiveAnyDamage`
  (params (Damage :type "Float (single-precision)") (DamageType :type "DamageType Object Reference") (InstigatedBy :type "Controller Object Reference") (DamageCauser :type "Actor Object Reference"))
  (bind _returnvalue (- (`self.CurrentHealth`) Damage))
  ;[1 1 1] GetDamage
  (if (<= _returnvalue 0.0)
    (`self.Death`)
    (else
      (set `self.CurrentHealth` _returnvalue))))

(event `StenWalk`
  (bind (_returnvalue_x _returnvalue_y _returnvalue_z) (`KismetMathLibrary.BreakVector` (`self.K2_GetActorLocation` self)))
  ;[1 1 1] RandomWalk
  (bind _returnvalue (`AIBlueprintHelperLibrary.GetAIController` self))
  (`AITask_MoveTo.AIMoveTo` _returnvalue (`KismetMathLibrary.MakeVector` (+ _returnvalue_x (`KismetMathLibrary.RandomFloatInRange` -2000.0 2000.0)) _returnvalue_y _returnvalue_z)
    (:`OnMoveFinished`
      (`self.StenWalk`))))

(event `self.CapsuleComponent.OnComponentBeginOverlap`
  (params (OverlappedComponent :type "PrimitiveComponent Object Reference") (OtherActor :type "Actor Object Reference") (OtherComp :type "PrimitiveComponent Object Reference") (OtherBodyIndex :type Integer) (bFromSweep :type Boolean) (SweepResult :type "HitResult Structure (by ref)"))
  ;[1 1 1] SetDamage
  (bind _askenny_character (cast `/Game/BluePrint/Character/KennyCharacter` OtherActor))
  (set `self.KennyChar` _askenny_character)
  (`self.PlayerInDamageZone`))

(event `self.CapsuleComponent.OnComponentEndOverlap`
  (params (OverlappedComponent :type "PrimitiveComponent Object Reference") (OtherActor :type "Actor Object Reference") (OtherComp :type "PrimitiveComponent Object Reference") (OtherBodyIndex :type Integer))
  ;[1 1 1] SetDamage
  (bind _askenny_character (cast `/Game/BluePrint/Character/KennyCharacter` OtherActor))
  (set `self.KennyChar` _askenny_character)
  (`self.PlayerNotInDamageZone`))

(event `PlayerInDamageZone`
  ;[1 1 1] SetDamage
  (`self.StartDamage`)
  (bind _returnvalue (`KismetSystemLibrary.K2_SetTimer` null "StartDamage" 1.0 true)))

(event `PlayerNotInDamageZone`
  ;[1 1 1] SetDamage
  (`KismetSystemLibrary.K2_ClearAndInvalidateTimerHandle` (stale `PlayerInDamageZone` _returnvalue)))

(fn `ChangeHealth`
  (if (<= (`self.CurrentHealth`) (`self.MaxHealth`))
    (set `self.CurrentHealth` (+ (`self.CurrentHealth`) (* (`GameplayStatics.GetWorldDeltaSeconds`) (`self.Regeneration`))))))

(fn `Death`
  (set `self.CurrentHealth` 0.0)
  (`self.K2_DestroyActor`))

(fn `Shot`
  (params (Damage :type "Float (double-precision)"))
  (returns (destroyBullet :type Boolean))
  ;[1 1 1] DamageFromBullet
  (return true))

(fn `StartDamage`
  (`GameplayStatics.ApplyDamage` (`self.KennyChar`) (`self.DamageSten`)))

(fn `UserConstructionScript`)