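; CailCharacter is a sprite character that wanders along the X axis under AI control.
; On BeginPlay it picks a random flipbook skin and walk speed.
; StenWalk sends AIMoveTo to a random X offset from its position and re-calls itself whether the move finishes or fails, giving endless roaming.
; Shot, marked as bullet damage, only returns true and ignores the damage value.
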(event `self.ReceiveBeginPlay`
  (`self.StenWalk`)
  ;[1 1 1] SetSkin
  (`PaperFlipbookComponent.SetFlipbook` (`self.Sprite`) (`KismetArrayLibrary.Array_Get` (`self.SpriteArray`) (`KismetMathLibrary.RandomIntegerInRange` 0 2)))
  ;[1 1 1] SpeedWalk
  (set `CharacterMovementComponent.MaxWalkSpeed` (`KismetMathLibrary.RandomFloatInRange` 20.0 100.0) (`self.CharacterMovement`)))

(event `StenWalk`
  (bind (_returnvalue_x _returnvalue_y _returnvalue_z) (`KismetMathLibrary.BreakVector` (`self.K2_GetActorLocation` self)))
  ;[1 1 1] RandomWalk
  (bind _returnvalue (`AIBlueprintHelperLibrary.GetAIController` self))
  (`AITask_MoveTo.AIMoveTo` _returnvalue (`KismetMathLibrary.MakeVector` (+ _returnvalue_x (`KismetMathLibrary.RandomFloatInRange` -2000.0 2000.0)) _returnvalue_y _returnvalue_z) null -1.0 "Default" "Default" true false
    (:`OnRequestFailed`
      _)
    (:`OnMoveFinished`
      _))
  (`self.StenWalk`))

(fn `Shot`
  (params (Damage :type "Float (double-precision)"))
  (returns (destroyBullet :type Boolean))
  ;[1 1 1] DamageFromBullet
  (return true))

(fn `UserConstructionScript`)