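; HUD Blueprint that draws a custom four-armed crosshair at the mouse position.
; Each DrawHUD call reads player 0's mouse position and offsets rectangles around it, leaving a gap at the center.
; Larger Color2 rectangles are drawn first, then smaller Color rectangles on top, giving each arm an outline.
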(event `self.ReceiveDrawHUD`
  (params (SizeX :type Integer) (SizeY :type Integer))
  (bind (_locationx _locationy) (`PlayerController.GetMousePosition` (`GameplayStatics.GetPlayerController` 0)))
  (set `self.LocMouseX` _locationx)
  (set `self.LocMouseY` _locationy)
  (`self.DrawRect` (`self.color2`) (+ (`self.LocMouseX`) 3.0) (- (`self.LocMouseY`) 1.0) 10.0 4.0)
  (`self.DrawRect` (`self.color2`) (- (`self.LocMouseX`) 1.0) (- (`self.LocMouseY`) 11.0) 4.0 10.0)
  (`self.DrawRect` (`self.color2`) (- (`self.LocMouseX`) 11.0) (+ (`self.LocMouseY`) -1.0) 10.0 4.0)
  (`self.DrawRect` (`self.color2`) (+ (`self.LocMouseX`) -1.0) (+ (`self.LocMouseY`) 3.0) 4.0 10.0)
  (`self.DrawRect` (`self.color`) (+ (`self.LocMouseX`) 4.0) (`self.LocMouseY`) 8.0 2.0)
  (`self.DrawRect` (`self.color`) (`self.LocMouseX`) (- (`self.LocMouseY`) 10.0) 2.0 8.0)
  (`self.DrawRect` (`self.color`) (- (`self.LocMouseX`) 10.0) (`self.LocMouseY`) 8.0 2.0)
  (`self.DrawRect` (`self.color`) (`self.LocMouseX`) (+ (`self.LocMouseY`) 4.0) 2.0 8.0))

(fn `UserConstructionScript`)